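; AI controller for BP_Enemy that runs BT_Enemy and feeds its blackboard the player's whereabouts and visibility.
; A looping timer drives data updates, writing the player's position even when unseen.
; Sight perception results are filtered of invalid, Enemy-tagged and dead actors.
; If the player remains, a fire-range trace ignoring fellow enemies sets the sight and range flags, while the pawn keeps facing the player.
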(event `Set Data`
  (bind _blackboard (`self.Blackboard`))
  (bind _target (`self.Target`))
  ;[1 0.6226 0.3307] Set Data
  (`|ExecutionSequence`
    (:`then_0`
      (`self.FilterTargets` (`AIPerceptionComponent.GetCurrentlyPerceivedActors` (`self.AIPerception`) "/Script/AIModule.AISense_Sight"))
      (`self.Target In Sight`))
    (:`then_1`
      (`/Engine/EditorBlueprintResources/StandardMacros.IsValid` _target
        (:`Is Valid`
          (`BlackboardComponent.SetValueAsVector` _blackboard "TargetPos" (`self.K2_GetActorLocation` _target)))))
    (:`then_2`
      (`/Engine/EditorBlueprintResources/StandardMacros.IsValid` _target
        (:`Is Valid`
          (`BlackboardComponent.SetValueAsObject` _blackboard "Player" (`GameplayStatics.GetPlayerPawn` 0)))))))

(event `Target Hittable`
  ;[1 1 1] Try to Hit Targets
  (bind _hit (`self.Fire Line Trace` (`/Game/Brackeys/Blueprints/BP_PlayerGamestate.Enemies` (`self.GameState`)) "TraceTypeQuery4" (`/Game/Brackeys/Blueprints/BP_Commando.FireRange` (`self.ControlledPawn`)) (`GameplayStatics.GetPlayerPawn` 0)))
  (set `self.CurrentTarget` (`.HitActor` (`GameplayStatics.BreakHitResult` _hit)))
  (`/Engine/EditorBlueprintResources/StandardMacros.IsValid` (`.HitActor` (`GameplayStatics.BreakHitResult` _hit))
    (:`Is Valid`
      (if (or (`self.ActorHasTag` (`ActorComponent.GetOwner` (`.HitComponent` (`GameplayStatics.BreakHitResult` _hit))) "Player") (`self.ActorHasTag` (`.HitActor` (`GameplayStatics.BreakHitResult` _hit)) "Player"))
        (`BlackboardComponent.SetValueAsBool` (`self.Blackboard`) "IsPlayerInSight" true)
        (`BlackboardComponent.SetValueAsBool` (`self.Blackboard`) "IsTargetInSight" true)
        (`self.Face Target` (`.HitActor` (`GameplayStatics.BreakHitResult` _hit)) (`self.ControlledPawn`))
        (`BlackboardComponent.SetValueAsBool` (`self.Blackboard`) "InRange" true)
        (else
          (`BlackboardComponent.SetValueAsBool` (`self.Blackboard`) "IsPlayerInSight" false :!label _label)
          (`BlackboardComponent.SetValueAsBool` (`self.Blackboard`) "IsTargetInSight" false)
          (`self.Face Target` (`GameplayStatics.GetPlayerPawn` 0) (`self.ControlledPawn`))
          (`BlackboardComponent.SetValueAsBool` (`self.Blackboard`) "InRange" false))))
    (:`Is Not Valid`
      (goto _label)))
  (`self.Face Target` (`GameplayStatics.GetPlayerPawn` 0) (`self.ControlledPawn`)))

(event `Target In Sight`
  ;[1 1 1] Check Targets
  (`self.FilterTargets` (`AIPerceptionComponent.GetCurrentlyPerceivedActors` (`self.AIPerception`) "/Script/AIModule.AISense_Sight"))
  (if (`KismetArrayLibrary.Array_Contains` (`self.Enemies`) (`GameplayStatics.GetPlayerPawn` 0))
    (`self.Target Hittable`)
    (else
      (`BlackboardComponent.SetValueAsBool` (`self.Blackboard`) "IsTargetInSight" false)
      (`BlackboardComponent.SetValueAsBool` (`self.Blackboard`) "IsPlayerInSight" false)
      (`BlackboardComponent.SetValueAsBool` (`self.Blackboard`) "InRange" false)
      (`self.Face Target` (`GameplayStatics.GetPlayerPawn` 0) (`self.ControlledPawn`))
      (set `self.CurrentTarget` null))))

(event `self.ReceiveBeginPlay`
  ;[1 1 1] Event Begin Play
  (`parent.ReceiveBeginPlay`)
  (`|ExecutionSequence`
    (:`then_0`
      (`KismetSystemLibrary.Delay` (`GameplayStatics.GetWorldDeltaSeconds`))
      (bind _asbp_enemy (cast `/Game/Brackeys/Blueprints/BP_Enemy` (`self.K2_GetPawn`)))
      (set `self.ControlledPawn` _asbp_enemy)
      (set `self.Target` (`GameplayStatics.GetPlayerPawn` 0)))
    (:`then_1`
      ;;[1 1 1] Run BT
      (`self.RunBehaviorTree` (`AIBlueprintHelperLibrary.GetAIController` self) "/Game/Brackeys/Blueprints/BT_Enemy.BT_Enemy"))
    (:`then_2`
      (bind _returnvalue (`KismetSystemLibrary.K2_SetTimerDelegate` (`|CreateDelegate` :!event `Set Data`) 0.2 true))
      (set `self.SetDataTimer` _returnvalue))))

(fn `FilterTargets`
  (params (Array :type "Array of Actor Object Reference"))
  (locals (`New Array` :type "Array of Actor Object Reference"))
  (set `self.Enemies` Array)
  (for _array_element (`self.Enemies`) :!label _label
    (`/Engine/EditorBlueprintResources/StandardMacros.IsValid` _array_element
      (:`Is Not Valid`
        (`KismetArrayLibrary.Array_RemoveItem` (`self.Enemies`) _array_element)
        (goto _label))))
  (for _array_element_2 (`self.Enemies`) :!label _label_2
    (if (`self.ActorHasTag` _array_element_2 "Enemy")
      (`KismetArrayLibrary.Array_RemoveItem` (`self.Enemies`) _array_element_2)
      (goto _label_2)))
  (for _array_element_3 (`self.Enemies`) :!label _label_3
    (bind _asbp_enemy (cast `/Game/Brackeys/Blueprints/BP_Enemy` _array_element_3))
    (if (`/Game/Brackeys/Blueprints/BP_Enemy.IsDead` _asbp_enemy)
      (`KismetArrayLibrary.Array_RemoveItem` (`self.Enemies`) _array_element_3)
      (goto _label_3))))

(fn `UserConstructionScript`)