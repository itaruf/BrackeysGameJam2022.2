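; BP_Spawnable is a spawnable actor with health and death handling, tracked among the game state's allies.
; It caches BP_PlayerGamestate on BeginPlay.
; Take Damage lowers clamped health and sends a death message when it reaches zero.
; The Death event fires an on-death event dispatcher, flags the actor as dead and removes it from the game state's Allies array.
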(event `self.ReceiveBeginPlay`
  (bind _asbp_player_gamestate (cast `/Game/Brackeys/Blueprints/BP_PlayerGamestate` (`GameplayStatics.GetGameState`)))
  (set `self.GameState` _asbp_player_gamestate))

(event `/Game/Brackeys/Blueprints/BPI_Health.Death`
  (bind _gamestate (`self.GameState`))
  (`self.EDI_OnDeath`)
  (set `self.IsDead` true)
  (`/Engine/EditorBlueprintResources/StandardMacros.IsValid` _gamestate
    (:`Is Valid`
      (`/Game/Brackeys/Blueprints/BP_PlayerGamestate.RemoveActor` _gamestate self (`/Game/Brackeys/Blueprints/BP_PlayerGamestate.Allies` (`self.GameState`))))))

(event `/Game/Brackeys/Blueprints/BPI_Damage.TakeDamage`
  (params (Value :type "Float (double-precision)"))
  ;[1 1 1] Take Damage
  (bind _output_get (set `self.Health` (`KismetMathLibrary.FClamp` (- (`self.Health`) Value) 0.0 (`self.MaxHealth`))))
  (if (<= _output_get 0.0)
    (message `/Game/Brackeys/Blueprints/BPI_Health.Death` self)))

(fn `UserConstructionScript`)