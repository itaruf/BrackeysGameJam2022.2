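; AI controller for the turret that runs BT_Turret and picks an enemy to aim at.
; A looping timer refreshes sight-perceived actors, filtering out invalid ones, players and dead enemies by restarting each loop after a removal.
; It line-traces toward the nearest one, faces an Enemy-tagged hit and sets IsTargetInSight on the Blackboard.
; The turret's death event sets IsDead and stops the timer.
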(event `Target Hittable`
  ;[1 1 1] Is Anything hittable
  (bind _hit (`self.Fire Line Trace` (`/Game/Brackeys/Blueprints/BP_PlayerGamestate.Allies` (`self.GameState`)) "TraceTypeQuery3" (`/Game/Brackeys/Blueprints/BP_Turret.FireRange` (`self.ControlledPawn`)) (`.ReturnValue` (`GameplayStatics.FindNearestActor` (`self.K2_GetActorLocation` (`self.ControlledPawn`)) (`self.Enemies`)))))
  (set `self.CurrentTarget` (`.HitActor` (`GameplayStatics.BreakHitResult` _hit)))
  (`/Engine/EditorBlueprintResources/StandardMacros.IsValid` (`.HitActor` (`GameplayStatics.BreakHitResult` _hit))
    (:`Is Valid`
      (if (`self.ActorHasTag` (`.HitActor` (`GameplayStatics.BreakHitResult` _hit)) "Enemy")
        (`BlackboardComponent.SetValueAsBool` (`self.Blackboard`) "IsTargetInSight" true)
        (bind _output_get (set `self.CurrentTarget` (`.HitActor` (`GameplayStatics.BreakHitResult` _hit))))
        (if (`KismetSystemLibrary.IsValid` _output_get)
          (`self.Face Target` (`self.CurrentTarget`) (`self.ControlledPawn`)))
        (else
          (`BlackboardComponent.SetValueAsBool` (`self.Blackboard`) "IsTargetInSight" false :!label _label)
          (set `self.CurrentTarget` null))))
    (:`Is Not Valid`
      (goto _label))))

(event `self.ReceiveBeginPlay`
  ;[1 1 1] Event Begin Play
  (`parent.ReceiveBeginPlay`)
  (`|ExecutionSequence`
    (:`then_0`
      (`KismetSystemLibrary.Delay` (`GameplayStatics.GetWorldDeltaSeconds`))
      (bind _asbp_turret (cast `/Game/Brackeys/Blueprints/BP_Turret` (`self.K2_GetPawn`)))
      (bind _output_get (set `self.ControlledPawn` _asbp_turret))
      (add `/Game/Brackeys/Blueprints/BP_Turret.EDI_OnDeath` _output_get (`|CreateDelegate` :!event `Set Values On Death`)))
    (:`then_1`
      (bind _returnvalue (`KismetSystemLibrary.K2_SetTimerDelegate` (`|CreateDelegate` :!event `Set Data`) 0.2 true))
      (set `self.SetDataTimer` _returnvalue))
    (:`then_2`
      ;;[1 1 1] Run BT
      (`self.RunBehaviorTree` (`AIBlueprintHelperLibrary.GetAIController` self) "/Game/Brackeys/Blueprints/BT_Turret.BT_Turret"))))

(event `Target In Sight`
  ;[1 1 1] Targets In Sight
  (if (>= (`KismetArrayLibrary.Array_Length` (`self.Enemies`)) 0)
    (`self.FilterTargets` (`AIPerceptionComponent.GetCurrentlyPerceivedActors` (`self.AIPerception`) "/Script/AIModule.AISense_Sight"))
    (`self.Target Hittable`)
    (else
      (`BlackboardComponent.SetValueAsBool` (`self.Blackboard`) "IsTargetInSight" false)
      (set `self.CurrentTarget` null))))

(event `self.ReceiveTick`
  (params (DeltaSeconds :type "Float (single-precision)")))

(event `Set Data`
  ;[1 1 1] Set Data
  (`/Engine/EditorBlueprintResources/StandardMacros.IsValid` (`self.Blackboard`)
    (:`Is Valid`
      (`|ExecutionSequence`
        (:`then_0`
          (`self.FilterTargets` (`AIPerceptionComponent.GetCurrentlyPerceivedActors` (`self.AIPerception`) "/Script/AIModule.AISense_Sight")))
        (:`then_1`
          (`self.Target In Sight`))))))

(event `Set Values On Death`
  ;[1 1 1] Set BB Values On Death
  (`BlackboardComponent.SetValueAsBool` (`self.Blackboard`) "IsDead" true)
  (`KismetSystemLibrary.K2_ClearAndInvalidateTimerHandle` (`self.SetDataTimer`)))

(fn `FilterTargets`
  (params (Array :type "Array of Actor Object Reference"))
  (set `self.Enemies` Array)
  (for _array_element (`self.Enemies`) :!label _label
    (`/Engine/EditorBlueprintResources/StandardMacros.IsValid` _array_element
      (:`Is Not Valid`
        (`KismetArrayLibrary.Array_RemoveItem` (`self.Enemies`) _array_element)
        (goto _label))))
  (for _array_element_2 (`self.Enemies`) :!label _label_2
    (if (`self.ActorHasTag` _array_element_2 "Player")
      (`KismetArrayLibrary.Array_RemoveItem` (`self.Enemies`) _array_element_2)
      (goto _label_2)))
  (for _array_element_3 (`self.Enemies`) :!label _label_3
    (bind _asbp_enemy (cast `/Game/Brackeys/Blueprints/BP_Enemy` _array_element_3))
    (if (`/Game/Brackeys/Blueprints/BP_Enemy.IsDead` _asbp_enemy)
      (`KismetArrayLibrary.Array_RemoveItem` (`self.Enemies`) _array_element_3)
      (goto _label_3))))

(fn `UserConstructionScript`)