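; BP_Healing is a temporary healing zone that restores health to a player standing inside it.
; On BeginPlay it plays a deploy sound, then destroys itself after ZoneDuration.
; When a BP_Player overlaps, it heals immediately through the player's CallEDIOnPlayerHeal dispatcher call and starts a looping timer for further ticks.
; Leaving the zone clears the in-zone flag and stops the HealingZone timer by function name.
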(event `self.ReceiveBeginPlay`
  (`GameplayStatics.PlaySoundAtLocation` "/Game/Brackeys/Audio/Sounds/HealZoneDeployedSound.HealZoneDeployedSound" (`SceneComponent.K2_GetComponentLocation` (`self.CollisionComponent`)) (struct) 1.0 1.0 0.0 null null null null)
  (`KismetSystemLibrary.Delay` (`self.ZoneDuration`))
  (`self.K2_DestroyActor`))

(event `self.ReceiveActorBeginOverlap`
  (params (OtherActor :type "Actor Object Reference"))
  (bind _asbp_player (cast `/Game/Brackeys/Blueprints/BP_Player` OtherActor))
  (set `self.PlayerRef` _asbp_player)
  (set `self.IsInHealingZone` true)
  (`self.HealingZone`)
  (`KismetSystemLibrary.K2_SetTimerDelegate` (`|CreateDelegate` :!event `HealingZone`) (`self.HealingTickDelay`) true))

(event `self.ReceiveActorEndOverlap`
  (params (OtherActor :type "Actor Object Reference"))
  (cast `/Game/Brackeys/Blueprints/BP_Player` OtherActor)
  (set `self.IsInHealingZone` false)
  (`KismetSystemLibrary.K2_ClearTimer` null "HealingZone"))

(event `HealingZone`
  (`/Game/Brackeys/Blueprints/BP_Player.EDI_OnPlayerHeal` (`self.PlayerRef`) (`self.HealingPower`)))

(fn `UserConstructionScript`)