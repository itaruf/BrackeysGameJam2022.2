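; BP_Commando is an AI-controlled combat character that handles fire cooldown, damage and death.
; TakeDamage clamps health, then either sends DeathMessage or briefly disables movement as a hit stagger.
; Death disables movement, switches collision to a dead profile and destroys the actor after a delay, while separate events update blackboard flags for its own or the player's death.
; CallEDI calls signal fire-stop, hit, recovery and death; DealDamage is empty.
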(event `self.ReceiveBeginPlay`
  ;[1 1 1] Event Begin Play
  (bind _asbp_player_gamestate (cast `/Game/Brackeys/Blueprints/BP_PlayerGamestate` (`GameplayStatics.GetGameState`)))
  (set `self.GameState` _asbp_player_gamestate))

(event `/Game/Brackeys/Blueprints/BPI_Fire.FireDelay`
  ;[1 1 1] Fire Delay
  (set `self.CanFire` false)
  (`self.EDI_OnStopFire`)
  (`KismetSystemLibrary.Delay` (`self.FireRate`))
  (set `self.CanFire` true))

(event `/Game/Brackeys/Blueprints/BPI_Damage.DealDamage`
  ;[1 1 1] Deal Damage
)

(event `/Game/Brackeys/Blueprints/BPI_Damage.TakeDamage`
  (params (Value :type "Float (double-precision)"))
  ;[1 1 1] Take Damage
  (bind _output_get (set `self.Health` (`KismetMathLibrary.FClamp` (- (`self.Health`) Value) 0.0 (`self.MaxHealth`))))
  (if (<= _output_get 0.0)
    (message `/Game/Brackeys/Blueprints/BPI_Health.Death` self)
    (else
      (`self.EDI_OnTakeDamage`)
      (`CharacterMovementComponent.DisableMovement` (`self.CharacterMovement`))
      (`KismetSystemLibrary.Delay` 0.1)
      (`CharacterMovementComponent.SetMovementMode` (`self.CharacterMovement`) "MOVE_Walking" 0)
      (`self.EDI_OnRecoverFromDamage`))))

(event `/Game/Brackeys/Blueprints/BPI_Health.Death`
  ;[1 1 1] Death
  (`self.EDI_OnDeath`)
  (`CharacterMovementComponent.DisableMovement` (`self.CharacterMovement`))
  (`PrimitiveComponent.SetCollisionObjectType` (`self.Mesh`) "ECC_GameTraceChannel8")
  (`PrimitiveComponent.SetCollisionProfileName` (`self.CapsuleComponent`) "Dead" true)
  (`PrimitiveComponent.SetCollisionResponseToChannel` (`self.CapsuleComponent`) "ECC_GameTraceChannel4" "ECR_Ignore")
  (`PrimitiveComponent.SetCollisionResponseToChannel` (`self.CapsuleComponent`) "ECC_GameTraceChannel5" "ECR_Ignore")
  (set `PrimitiveComponent.bGenerateOverlapEvents` false (`self.CapsuleComponent`))
  (`PrimitiveComponent.SetCollisionProfileName` (`self.CapsuleComponent`) "Dead" true)
  (`KismetSystemLibrary.Delay` 3.0)
  (`self.K2_DestroyActor`))

(event `Set Values On Death`
  (bind _returnvalue (`AIBlueprintHelperLibrary.GetAIController` self))
  ;[1 1 1] Death Events
  (set `self.IsDead` true)
  (`BlackboardComponent.SetValueAsBool` (`AIController.Blackboard` _returnvalue) "IsTargetInSight" false)
  (`BlackboardComponent.SetValueAsBool` (`AIController.Blackboard` _returnvalue) "IsPlayerInSight" false)
  (`BlackboardComponent.SetValueAsBool` (`AIController.Blackboard` _returnvalue) "IsDead" true))

(event `Set Values On Player Death`
  (bind _returnvalue (`AIBlueprintHelperLibrary.GetAIController` self))
  ;[1 1 1] Death Events
  (`BlackboardComponent.SetValueAsBool` (`AIController.Blackboard` _returnvalue) "IsTargetInSight" false)
  (`BlackboardComponent.SetValueAsBool` (`AIController.Blackboard` _returnvalue) "IsPlayerInSight" false)
  (`BlackboardComponent.SetValueAsBool` (`AIController.Blackboard` _returnvalue) "IsPlayerDead" true))

(fn `UserConstructionScript`)