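; BP_Wave spawns one enemy wave, placing units at spawn points taken from the game state's WaveTargetPoints map, facing the player.
; After an initial delay, a looping timer spawns units with default controllers until the WaveData enemy count is reached.
; GetValidSpawnPoint re-rolls randomly at each read, so the point it marks used can differ from the one returned.
; A counter periodically triggers ClearSpawnPoints, which returns after unmarking the first point.
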(event `self.ReceiveBeginPlay`
  (bind (_wavedata_nbenemies _wavedata_spawndelay) (break `/Game/Brackeys/Blueprints/S_WaveData` (`self.WaveData`)))
  (`KismetSystemLibrary.Delay` (`GameplayStatics.GetWorldDeltaSeconds`))
  (`|ExecutionSequence`
    (:`then_0`
      (bind _asbp_player_gamestate (cast `/Game/Brackeys/Blueprints/BP_PlayerGamestate` (`GameplayStatics.GetGameState`)))
      (bind _output_get (set `self.GameState` _asbp_player_gamestate))
      (bind _keys (`BlueprintMapLibrary.Map_Keys` (`/Game/Brackeys/Blueprints/BP_PlayerGamestate.WaveTargetPoints` _output_get)))
      (set `self.SpawnPoints` _keys)
      (`self.GetClearCounter`))
    (:`then_1`
      (`KismetSystemLibrary.Delay` _wavedata_spawndelay)
      (bind _returnvalue (`KismetSystemLibrary.K2_SetTimerDelegate` (`|CreateDelegate` :!event `Spawn Wave`) (`self.SpawnDelayPerUnit`) true))
      (set `self.SpawnWaveTimer` _returnvalue))))

(event `Spawn Wave`
  (bind _wavedata_nbenemies (break `/Game/Brackeys/Blueprints/S_WaveData` (`self.WaveData`)))
  (if (< (`self.SpawnCounter`) _wavedata_nbenemies)
    (`/Engine/EditorBlueprintResources/StandardMacros.IncrementInt` (`self.C`)
      (:`  `
        (if (== (`self.C`) (+ (`self.Counter`) 1))
          (`self.ClearSpawnPoints`)
          (else
            (`/Engine/EditorBlueprintResources/StandardMacros.IncrementInt` (`self.SpawnCounter`)
              (:`  `
                (bind _spawnpoint (`self.GetValidSpawnPoint`))
                (set `self.SpawnPoint` _spawnpoint)
                (bind _returnvalue (`|SpawnActorFromClass` (`self.Spawned`) (`KismetMathLibrary.MakeTransform` (`self.K2_GetActorLocation` (`self.SpawnPoint`)) (`KismetMathLibrary.FindLookAtRotation` (`self.K2_GetActorLocation` (`self.SpawnPoint`)) (`self.K2_GetActorLocation` (`GameplayStatics.GetPlayerPawn` 0)))) "Undefined" "OverrideRootScale" null null))
                (`Pawn.SpawnDefaultController` _returnvalue)))))))
    (else
      (`KismetSystemLibrary.K2_ClearAndInvalidateTimerHandle` (`self.SpawnWaveTimer`)))))

(fn `ClearSpawnPoints`
  (for _array_element (`self.SpawnPoints`)
    (`BlueprintMapLibrary.Map_Add` (`/Game/Brackeys/Blueprints/BP_PlayerGamestate.WaveTargetPoints` (`self.GameState`)) _array_element)
    (return))
  (set `self.C` 0))

(fn `GetClearCounter`
  (bind _wavedata_nbenemies (break `/Game/Brackeys/Blueprints/S_WaveData` (`self.WaveData`)))
  (bind _wavedata_nbenemies_2 (break `/Game/Brackeys/Blueprints/S_WaveData` (`self.WaveData`)))
  (bind _wavedata_nbenemies_3 (break `/Game/Brackeys/Blueprints/S_WaveData` (`self.WaveData`)))
  (if (> _wavedata_nbenemies_3 (`KismetArrayLibrary.Array_Length` (`self.SpawnPoints`)))
    (set `self.Counter` (`KismetMathLibrary.FCeil` (`KismetMathLibrary.Conv_IntToDouble` (/ _wavedata_nbenemies (`KismetArrayLibrary.Array_Length` (`self.SpawnPoints`))))))
    (else
      (set `self.Counter` _wavedata_nbenemies_2))))

(fn `GetValidSpawnPoint`
  (returns (SpawnPoint :type "/Game/Brackeys/Blueprints/BP_WaveTargetPoint Object Reference"))
  (bind _outitem (`KismetArrayLibrary.Array_Random` (`self.SpawnPoints`)))
  (bind _wavetargetpoints (`/Game/Brackeys/Blueprints/BP_PlayerGamestate.WaveTargetPoints` (`self.GameState`)))
  (if (not (`BlueprintMapLibrary.Map_Find` _wavetargetpoints _outitem))
    (`BlueprintMapLibrary.Map_Add` _wavetargetpoints _outitem true))
  (return _outitem))

(fn `UserConstructionScript`)