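; BP_Ally is an AI-controlled ally character that shoots projectiles at targets, extending a parent class's begin play and death logic.
; BeginPlay caches its BP_AllyController and the player, then binds to death dispatchers.
; Fire launches a BP_Projectile at an in-range target, or clears the blackboard's IsTargetInSight when the target is invalid.
; Death removes it from GameState's Allies, and death handlers stop the controller's SetDataTimer.
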(event `self.ReceiveBeginPlay`
  ;[1 1 1] Event Begin Play
  (`parent.ReceiveBeginPlay`)
  (`|ExecutionSequence`
    (:`then_0`
      (`KismetSystemLibrary.Delay` (`GameplayStatics.GetWorldDeltaSeconds`))
      (bind _asbp_ally_controller (cast `/Game/Brackeys/Blueprints/BP_AllyController` (`AIBlueprintHelperLibrary.GetAIController` self)))
      (set `self.AllyController` _asbp_ally_controller))
    (:`then_1`
      (`self.Set Values`)
      (bind _asbp_player (cast `/Game/Brackeys/Blueprints/BP_Player` (`GameplayStatics.GetPlayerPawn` 0)))
      (bind _output_get (set `self.Player` _asbp_player))
      (add `/Game/Brackeys/Blueprints/BP_Player.EDI_OnDeath` _output_get (`|CreateDelegate` :!event `Set Values On Player Death`))
      (add `self.EDI_OnDeath` (`|CreateDelegate` :!event `Set Values On Death`)))
    (:`then_2`
      (`GameplayStatics.PlaySoundAtLocation` "/Game/Brackeys/Audio/Sounds/Utilities-Sensor-02.Utilities-Sensor-02" (`SceneComponent.K2_GetComponentLocation` (`self.Mesh`)) (struct) 1.0 1.0 0.0 null null null null))))

(event `self.Set Values On Death`
  (`parent.Set Values On Death`)
  (`KismetSystemLibrary.K2_ClearAndInvalidateTimerHandle` (`/Game/Brackeys/Blueprints/BP_AIController.SetDataTimer` (`self.AllyController`)) :!label _label))

(event `self.Set Values On Player Death`
  (`parent.Set Values On Player Death`)
  (goto _label))

(event `/Game/Brackeys/Blueprints/BPI_Fire.Fire`
  (params (Target :type "Actor Object Reference"))
  ;[1 1 1] Fire
  (`/Engine/EditorBlueprintResources/StandardMacros.IsValid` Target
    (:`Is Valid`
      (bind _output_get (set `self.CurrentTarget` Target))
      (if (`self.CanFire`)
        (`self.EDI_OnFire`)
        (if (<= (`KismetMathLibrary.Vector_Distance` (`self.K2_GetActorLocation`) (`self.K2_GetActorLocation` _output_get)) (`self.FireRange`))
          (bind _returnvalue (`|SpawnActorFromClass` "/Game/Brackeys/Blueprints/BP_Projectile.BP_Projectile_C" (`KismetMathLibrary.MakeTransform` (`SceneComponent.K2_GetComponentLocation` (`self.ProjectileSpawn`)) (struct) (0.1 0.1 0.1)) "Undefined" "OverrideRootScale" null null))
          (`GameplayStatics.PlaySoundAtLocation` "/Game/Brackeys/Audio/Sounds/Resistance-AssaultRifle_03-Single_Shot-04.Resistance-AssaultRifle_03-Single_Shot-04" (0.0 0.0 0.0) (struct) 0.2 1.0 0.0 null null null null)
          (set `/Game/Brackeys/Blueprints/BP_Projectile.Damage` (`self.FireDamage`) _returnvalue)
          (`/Game/Brackeys/Blueprints/BP_Projectile.On Spawn` _returnvalue (* (`KismetMathLibrary.GetForwardVector` (`KismetMathLibrary.FindLookAtRotation` (`self.K2_GetActorLocation`) (`self.K2_GetActorLocation` (`self.CurrentTarget`)))) 2000.0) "/Game/Brackeys/Blueprints/BP_Enemy.BP_Enemy_C" "ECC_GameTraceChannel4" false 1.0)
          (message `/Game/Brackeys/Blueprints/BPI_Fire.FireDelay` self))))
    (:`Is Not Valid`
      (`BlackboardComponent.SetValueAsBool` (`AIController.Blackboard` (`self.AllyController`)) "IsTargetInSight" false))))

(event `/Game/Brackeys/Blueprints/BPI_Health.Death`
  ;[1 1 1] Event Death
  (`parent.Death`)
  (`/Game/Brackeys/Blueprints/BP_PlayerGamestate.RemoveActor` (`self.GameState`) self (`/Game/Brackeys/Blueprints/BP_PlayerGamestate.Allies` (`self.GameState`))))

(fn `FireLineTraceDebug`
  (bind _returnvalue (`self.K2_GetActorLocation`))
  (bind _outactors (`GameplayStatics.GetAllActorsOfClass` "/Game/Brackeys/Blueprints/BP_Enemy.BP_Enemy_C"))
  (`KismetSystemLibrary.LineTraceSingle` _returnvalue (+ _returnvalue (* (`KismetMathLibrary.GetForwardVector` (`KismetMathLibrary.FindLookAtRotation` (`self.K2_GetActorLocation`) (`self.K2_GetActorLocation` (`self.CurrentTarget`)))) (`self.FireRange`))) "TraceTypeQuery2" true _outactors "ForDuration" true (struct :`G` 0.758331 :`B` 1.0 :`A` 1.0) (struct :`G` 1.0 :`A` 1.0) (`self.FireRate`)))

(fn `FireLineTraceTrack`
  (returns (Hit :type "HitResult Structure") (ReturnValue :type Boolean))
  (bind _returnvalue (`self.K2_GetActorLocation`))
  (bind _outactors (`GameplayStatics.GetAllActorsOfClass` "/Game/Brackeys/Blueprints/BP_Enemy.BP_Enemy_C"))
  (bind (_outhit _returnvalue_2) (`KismetSystemLibrary.LineTraceSingle` _returnvalue (+ _returnvalue (* (`KismetMathLibrary.GetForwardVector` (`KismetMathLibrary.FindLookAtRotation` (`self.K2_GetActorLocation`) (`self.K2_GetActorLocation` (`GameplayStatics.GetPlayerPawn` 0)))) (`self.FireRange`))) "TraceTypeQuery2" true _outactors "ForDuration" true (struct :`R` 1.0 :`B` 0.002399 :`A` 1.0) (struct :`G` 1.0 :`A` 1.0) 0.5))
  (return _outhit _returnvalue_2))

(fn `Set Values`
  (`|ExecutionSequence`
    (:`then_0`
      (set `self.MaxHealth` (`self.Health`)))
    (:`then_1`
      (bind _asbp_player (cast `/Game/Brackeys/Blueprints/BP_Player` (`GameplayStatics.GetPlayerPawn` 0)))
      (set `self.Player` _asbp_player))))

(fn `UserConstructionScript`)