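; BP_PlayerGamestate holds shared match state: allies, enemies, wave target points, pause status, and the game-ended and won flags.
; BeginPlay registers the player pawn as an ally and maps every BP_WaveTargetPoint in the level to false.
; Events update the pause and result flags.
; Tick scans Allies and Enemies for invalid actors, though ClearArray always removes from Enemies, so invalid allies remain.
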(event `self.ReceiveBeginPlay`
  (`|ExecutionSequence`
    (:`then_1`
      (`KismetArrayLibrary.Array_AddUnique` (`self.Allies`) (`GameplayStatics.GetPlayerPawn` 0))
      (bind _outactors (`GameplayStatics.GetAllActorsOfClass` "/Game/Brackeys/Blueprints/BP_WaveTargetPoint.BP_WaveTargetPoint_C"))
      (for _array_element _outactors
        (`BlueprintMapLibrary.Map_Add` (`self.WaveTargetPoints`) _array_element)))))

(event `OnGameEnded`
  (params (IsGameWon :type Boolean))
  (set `self.GameIsWon` IsGameWon)
  (set `self.GameEnded` true))

(event `UpdatePauseStatus`
  (params (IsPaused :type Boolean))
  (set `self.IsPaused` IsPaused))

(event `self.ReceiveTick`
  (params (DeltaSeconds :type "Float (single-precision)"))
  (`self.ClearArray` (`self.Allies`))
  (`self.ClearArray` (`self.Enemies`)))

(fn `ClearArray`
  (params (Array :type "Array of Actor Object Reference"))
  (for _array_element Array
    (`/Engine/EditorBlueprintResources/StandardMacros.IsValid` _array_element
      (:`Is Not Valid`
        (`KismetArrayLibrary.Array_RemoveItem` (`self.Enemies`) _array_element)))))

(fn `RemoveActor`
  (params (Actor :type "Actor Object Reference") (Array :type "Array of Actor Object Reference"))
  (`KismetArrayLibrary.Array_RemoveItem` Array Actor))

(fn `UserConstructionScript`)