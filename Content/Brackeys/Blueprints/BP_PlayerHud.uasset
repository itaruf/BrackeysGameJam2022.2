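; BP_PlayerHud builds the player's on-screen UI: countdown timer, health bar, power buttons and crosshair.
; Power buttons are enabled or disabled by index through an event bound to BP_Player.
; When GameDuration elapses, a looping timer replays a timeline whose FlipFlop flashes the win/lose result widget.
; SetResult marks the game lost, shows the result and removes the gameplay widgets, then the timer after a delay.
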(event `self.ReceiveBeginPlay`
  (bind _powerswidgetref (`self.PowersWidgetRef`))
  (`|ExecutionSequence`
    (:`then_1`
      ;[1 1 1] Display timer
      (bind _returnvalue (`|GenericCreateObject` "/Game/Brackeys/Widgets/BP_TimeWidget.BP_TimeWidget_C" (`self.GameDuration`)))
      (bind _output_get (set `self.TimerWidgetRef` _returnvalue))
      (`UserWidget.AddToViewport` _output_get 0)
      (`KismetSystemLibrary.Delay` (`self.GameDuration`))
      (`Widget.RemoveFromParent` (`self.TimerWidgetRef`))
      (bind _returnvalue_2 (`KismetSystemLibrary.K2_SetTimerDelegate` (delegate `DisplayResult`) 0.6 true))
      (set `self.DisplayResultTimer` _returnvalue_2)
      ;[1 1 1] Display result alert
      (`Timeline|Timeline_0` :!label _label
        (:`Update`
          (`KismetSystemLibrary.Delay` 0.5)
          (`/Engine/EditorBlueprintResources/StandardMacros.FlipFlop`
            (:`A`
              (bind _returnvalue_3 (`|CreateWidget` "/Game/Brackeys/Widgets/BP_ResultWidget.BP_ResultWidget_C" null (`self.IsGameWon`)))
              (`UserWidget.AddToViewport` _returnvalue_3 0))
            (:`B`
              (`Widget.RemoveFromParent` _returnvalue_3))))))
    (:`then_2`
      (bind _returnvalue_4 (`|GenericCreateObject` "/Game/Brackeys/Widgets/BP_HealthBarWidget.BP_HealthBarWidget_C"))
      (bind _output_get_2 (set `self.HealthBarWidgetRef` _returnvalue_4))
      (`UserWidget.AddToViewport` _output_get_2 0))
    (:`then_3`
      (`self.BuildPowerWidget`)
      (set `self.BtnArray` (`|MakeArray` (`/Game/Brackeys/Widgets/BP_PowersWidget.BtnHeal` _powerswidgetref) (`/Game/Brackeys/Widgets/BP_PowersWidget.BtnTurret` _powerswidgetref) (`/Game/Brackeys/Widgets/BP_PowersWidget.BtnFreeze` _powerswidgetref) (`/Game/Brackeys/Widgets/BP_PowersWidget.BtnAlly` _powerswidgetref))))
    (:`then_4`
      (bind _returnvalue_5 (`|GenericCreateObject` "/Game/Brackeys/Widgets/BP_CrosshairWidget.BP_CrosshairWidget_C"))
      (bind _output_get_3 (set `self.CrossHairWidgetRef` _returnvalue_5))
      (`UserWidget.AddToViewport` _output_get_3 0))
    (:`then_5`
      (bind _asbp_player (cast `/Game/Brackeys/Blueprints/BP_Player` (`GameplayStatics.GetPlayerPawn` 0)))
      (add `/Game/Brackeys/Blueprints/BP_Player.EDI_OnPowersAvailablity` _asbp_player (`|CreateDelegate` :!event `Update Powers Availability`)))))

(event `DisplayResult`
  (goto _label))

(event `Set Result`
  (set `self.IsGameWon` false)
  (`self.DisplayResult`)
  (`KismetSystemLibrary.K2_ClearAndInvalidateTimerHandle` (`self.DisplayResultTimer`))
  (`Widget.RemoveFromParent` (`self.PowersWidgetRef`))
  (`Widget.RemoveFromParent` (`self.HealthBarWidgetRef`))
  (`Widget.RemoveFromParent` (`self.CrossHairWidgetRef`))
  (`KismetSystemLibrary.Delay` 5.0)
  (`Widget.RemoveFromParent` (`self.TimerWidgetRef`)))

(event `Update Powers Availability`
  (params (IsAvailable :type Boolean) (ButtonId :type Integer))
  (`Widget.SetIsEnabled` (`|GetArrayItem` (`self.BtnArray`) ButtonId) IsAvailable))

(event `Add Power Widget`
  ;[1 1 1] Add Power Widget
  (`/Engine/EditorBlueprintResources/StandardMacros.IsValid` (`self.PowersWidgetRef`)
    (:`Is Valid`
      (if (not (`Widget.IsVisible` (`self.PowersWidgetRef`)))
        (`UserWidget.AddToViewport` (`self.PowersWidgetRef`) 0)))))

(fn `BuildPowerWidget`
  (bind _returnvalue (`|GenericCreateObject` "/Game/Brackeys/Widgets/BP_PowersWidget.BP_PowersWidget_C"))
  (bind _output_get (set `self.PowersWidgetRef` _returnvalue))
  (`UserWidget.AddToViewport` _output_get 0))

(fn `UserConstructionScript`)