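; BP_EnemyProjectile is a physics-driven enemy projectile that deals damage to whatever it hits through BPI_Damage.
; A custom spawn event launches the mesh by impulse scaled by inverse FreezeStrength, sets its collision object type and, when Dilated, slows the actor's time dilation.
; Damaging hits swap the projectile effect for a hit effect before delayed destruction; other hits destroy it immediately.
; The spawner-exclusion check is disconnected.
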(event `self.ReceiveBeginPlay`
  (`parent.ReceiveBeginPlay`))

(event `CustomEvent`
  (params (Impulse :type "Vector Structure") (Spawner :type "Actor Class Reference") (CollisionChannel :type "ECollisionChannel Enum" :default "ECC_WorldStatic") (Dilated :type Boolean) (FreezeStrength :type "Float (double-precision)" :default 1.0))
  ;[1 1 1] On Spawn
  (`|ExecutionSequence`
    (:`then_0`
      (if Dilated
        (bind _output_get (set `self.CustomTimeDilation` (/ 1.0 FreezeStrength)))
        (`KismetSystemLibrary.PrintString` (`KismetStringLibrary.Conv_DoubleToString` _output_get))))
    (:`then_1`
      (`PrimitiveComponent.AddImpulse` (`self.StaticMesh`) (* Impulse (/ 1.0 FreezeStrength)) "None" true))
    (:`then_2`
      (set `self.Spawner` Spawner)
      (`PrimitiveComponent.SetCollisionObjectType` (`self.StaticMesh`) CollisionChannel))))

(event `self.ReceiveHit`
  (params (MyComp :type "PrimitiveComponent Object Reference") (Other :type "Actor Object Reference") (OtherComp :type "PrimitiveComponent Object Reference") (bSelfMoved :type Boolean) (HitLocation :type "Vector Structure") (HitNormal :type "Vector Structure") (NormalImpulse :type "Vector Structure") (Hit :type "HitResult Structure (by ref)"))
  (bind _hiteffect (`self.HitEffect`))
  (bind _asbpi_damage (cast `/Game/Brackeys/Blueprints/BPI_Damage` Other)
    (:`then`
      (message `/Game/Brackeys/Blueprints/BPI_Damage.TakeDamage` (`KismetSystemLibrary.Conv_InterfaceToObject` _asbpi_damage) (`self.Damage`))
      (`ActorComponent.Deactivate` (`self.ProjectileEffect`))
      (`ActorComponent.SetActive` _hiteffect true false)
      (`SceneComponent.K2_SetWorldLocation` _hiteffect HitLocation false false)
      (`KismetSystemLibrary.Delay` 1.0)
      (`self.K2_DestroyActor`))
    (:`CastFailed`
      (`self.K2_DestroyActor`))))

(fn `UserConstructionScript`
  (`parent.UserConstructionScript`))