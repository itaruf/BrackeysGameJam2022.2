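; BP_Turret is a turret pawn that shoots projectiles at a target passed to its Fire event, caching its BP_TurretController after BeginPlay.
; Fire checks validity, cooldown and range, then spawns a damage-carrying BP_Projectile launched toward the target from ProjectileSpawn.
; A FireDelay event gates the fire rate, and Death switches collision to a dead profile.
; FireLineTraceDebug draws a debug trace toward the current target, ignoring spawnables and the player.
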(event `self.ReceiveBeginPlay`
  ;[1 1 1] Begin Play
  (`KismetSystemLibrary.Delay` (`GameplayStatics.GetWorldDeltaSeconds`))
  (bind _asbp_turret_controller (cast `/Game/Brackeys/Blueprints/BP_TurretController` (`self.GetController`)))
  (set `self.TurretController` _asbp_turret_controller))

(event `/Game/Brackeys/Blueprints/BPI_Health.Death`
  ;[1 1 1] Death
  (`parent.Death`)
  (`PrimitiveComponent.SetCollisionObjectType` (`self.StaticMesh`) "ECC_GameTraceChannel8")
  (`PrimitiveComponent.SetCollisionProfileName` (`self.Capsule`) "Dead" true)
  (`PrimitiveComponent.SetCollisionResponseToChannel` (`self.Capsule`) "ECC_GameTraceChannel4" "ECR_Ignore")
  (`PrimitiveComponent.SetCollisionResponseToChannel` (`self.Capsule`) "ECC_GameTraceChannel5" "ECR_Ignore")
  (set `PrimitiveComponent.bGenerateOverlapEvents` false (`self.Capsule`))
  (`PrimitiveComponent.SetCollisionProfileName` (`self.Capsule`) "Dead" true))

(event `/Game/Brackeys/Blueprints/BPI_Fire.Fire`
  (params (Target :type "Actor Object Reference"))
  ;[1 1 1] Fire
  (`/Engine/EditorBlueprintResources/StandardMacros.IsValid` Target
    (:`Is Valid`
      (set `self.CurrentTarget` Target)
      (if (`self.CanFire`)
        (if (<= (`KismetMathLibrary.Vector_Distance` (`self.K2_GetActorLocation`) (`self.K2_GetActorLocation` Target)) (`self.FireRange`))
          (bind _returnvalue (`|SpawnActorFromClass` "/Game/Brackeys/Blueprints/BP_Projectile.BP_Projectile_C" (`KismetMathLibrary.MakeTransform` (`SceneComponent.K2_GetComponentLocation` (`self.ProjectileSpawn`)) (struct) (0.1 0.1 0.1)) "Undefined" "OverrideRootScale" null null))
          (set `/Game/Brackeys/Blueprints/BP_Projectile.Damage` (`self.FireDamage`) _returnvalue)
          (`/Game/Brackeys/Blueprints/BP_Projectile.On Spawn` _returnvalue (* (`KismetMathLibrary.GetForwardVector` (`KismetMathLibrary.FindLookAtRotation` (`SceneComponent.K2_GetComponentLocation` (`self.ProjectileSpawn`)) (`self.K2_GetActorLocation` (`self.CurrentTarget`)))) 2500.0) "BP_Turret_C" "ECC_GameTraceChannel4" false 1.0)
          (message `/Game/Brackeys/Blueprints/BPI_Fire.FireDelay` self))))))

(event `/Game/Brackeys/Blueprints/BPI_Fire.FireDelay`
  ;[1 1 1] Fire Delay
  (set `self.CanFire` false)
  (`KismetSystemLibrary.Delay` (`self.FireRate`))
  (set `self.CanFire` true))

(fn `FireLineTraceDebug`
  (bind _returnvalue (`self.K2_GetActorLocation`))
  (`/Engine/EditorBlueprintResources/StandardMacros.IsValid` (`self.CurrentTarget`)
    (:`Is Valid`
      (`KismetArrayLibrary.Array_Clear` (`self.Actors to Ignore`))
      (bind _outactors (`GameplayStatics.GetAllActorsOfClass` "/Game/Brackeys/Blueprints/BP_Spawnable.BP_Spawnable_C"))
      (bind _output_get (set `self.Actors to Ignore` _outactors))
      (`KismetArrayLibrary.Array_Add` _output_get (`GameplayStatics.GetPlayerPawn` 0))
      (`KismetSystemLibrary.LineTraceSingle` _returnvalue (+ _returnvalue (* (`KismetMathLibrary.GetForwardVector` (`KismetMathLibrary.FindLookAtRotation` (`self.K2_GetActorLocation`) (`self.K2_GetActorLocation` (`self.CurrentTarget`)))) (`self.FireRange`))) "TraceTypeQuery2" true (`self.Actors to Ignore`) "ForDuration" true (struct :`A` 1.0) (struct :`G` 1.0 :`A` 1.0) (`self.FireRate`)))))

(fn `UserConstructionScript`
  (`parent.UserConstructionScript`))