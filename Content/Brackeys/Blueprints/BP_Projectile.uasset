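; Physics-driven projectile that is launched by impulse, damages what it hits and has a limited lifespan.
; OnSpawn sets collision channel and spawner, scales the impulse by inverse FreezeStrength and, if Dilated, slows its own time by that factor.
; Hits on anything not matching the spawner's class send damage through BPI_Damage, stop physics and collision, and show an impact effect before destruction.
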(event `self.ReceiveBeginPlay`
  ;[1 1 1] Begin Play
  (`self.SetLifeSpan` (`self.Lifespan`))
  (`NiagaraComponent.SetAsset` (`self.ProjectileEffect`) (`self.ProjectileFX`) true)
  (`NiagaraComponent.SetAsset` (`self.HitEffect`) (`self.HitEffectFX`) true)
  (`ActorComponent.Deactivate` (`self.MuzzleEffect`)))

(event `On Spawn`
  (params (Impulse :type "Vector Structure") (Spawner :type "Actor Class Reference") (CollisionChannel :type "ECollisionChannel Enum" :default "ECC_WorldStatic") (Dilated :type Boolean) (FreezeStrength :type "Float (double-precision)" :default 1.0))
  ;[1 1 1] On Spawn
  (`|ExecutionSequence`
    (:`then_0`
      (if Dilated
        (set `self.CustomTimeDilation` (/ 1.0 FreezeStrength))
        (`PrimitiveComponent.SetCollisionObjectType` (`self.Sphere`) CollisionChannel)
        (`PrimitiveComponent.SetCollisionObjectType` (`self.StaticMesh`) CollisionChannel)))
    (:`then_1`
      (`PrimitiveComponent.AddImpulse` (`self.StaticMesh`) (* Impulse (/ 1.0 FreezeStrength)) "None" true))
    (:`then_2`
      (set `self.Spawner` Spawner)
      (`PrimitiveComponent.SetCollisionObjectType` (`self.StaticMesh`) CollisionChannel))))

(event `self.ReceiveHit`
  (params (MyComp :type "PrimitiveComponent Object Reference") (Other :type "Actor Object Reference") (OtherComp :type "PrimitiveComponent Object Reference") (bSelfMoved :type Boolean) (HitLocation :type "Vector Structure") (HitNormal :type "Vector Structure") (NormalImpulse :type "Vector Structure") (Hit :type "HitResult Structure (by ref)"))
  (bind _hiteffect (`self.HitEffect`))
  (if (!= (`GameplayStatics.GetObjectClass` Other) (`self.Spawner`))
    (bind _asbpi_damage (cast `/Game/Brackeys/Blueprints/BPI_Damage` Other)
      (:`then`
        (message `/Game/Brackeys/Blueprints/BPI_Damage.TakeDamage` (`KismetSystemLibrary.Conv_InterfaceToObject` _asbpi_damage) (`self.Damage`)))
      (:`CastFailed`
        _))
    (`ActorComponent.Deactivate` (`self.ProjectileEffect`))
    (`PrimitiveComponent.SetSimulatePhysics` (`self.StaticMesh`) false)
    (`PrimitiveComponent.SetCollisionEnabled` (`self.Sphere`) "NoCollision")
    (`PrimitiveComponent.SetCollisionEnabled` (`self.StaticMesh`) "NoCollision")
    (`ActorComponent.SetActive` _hiteffect true false)
    (`SceneComponent.K2_SetWorldLocation` _hiteffect Hit_ImpactPoint false false)
    (`KismetSystemLibrary.Delay` 0.1)
    (`self.K2_DestroyActor`)))

(fn `UserConstructionScript`)